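; Dialog actor that shows a devil-themed widget alongside a dialog box.
; DisplayDialog creates and displays a Devil_2 widget, then a Dialog_WBP that receives DialogText and a reference back to this actor as its parent.
; The Construction Script mirrors DialogText onto the DialogActorText component.
; When the actor is destroyed, it removes the Devil_2 widget but leaves the dialog widget untouched.
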(event EventBeginPlay)

(event Collision|EventActorBeginOverlap
  (params (OtherActor :type Actor%20Object%20Reference)))

(event EventTick
  (params (DeltaSeconds :type Float%20%28single-precision%29)))

(event EventDisplayDialog
  (bind _returnvalue (UserInterface|CreateWidget "/Game/UserInterface/Devil_2.Devil_2_C"))
  (bind _output_get (Variables|Default|SetNewVar _returnvalue))
  (UserInterface|Viewport|AddtoViewport _output_get 0)
  (bind _returnvalue_2 (UserInterface|CreateWidget "/Game/UserInterface/Dialog_WBP.Dialog_WBP_C"))
  (bind _output_get_2 (Variables|Default|SetDialogWidget _returnvalue_2))
  (Default|SetDialogText _output_get_2 (Variables|Default|GetDialogText))
  (Variables|/Game/UserInterface/Dialog_WBP.Dialog_WBP_C|SetDialogParent _output_get_2 self)
  (UserInterface|Viewport|AddtoViewport _output_get_2 0))

(event EventDestroyed
  (Widget|RemovefromParent (stale EventDisplayDialog _output_get)))

(fn ConstructionScript
  (Rendering|Components|TextRender|SetText (Variables|Default|GetDialog%20actor%20text) (Utilities|Text|ToText(String) (Variables|Default|GetDialogText))))